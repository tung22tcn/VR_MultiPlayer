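; Game instance Blueprint that hosts and searches for multiplayer sessions, over LAN or internet.
; CreateRoom stores the player limit and LAN flag, creates a session, then opens FirstPersonExampleMap as a listen server.
; FindRoom searches with those stored values, reusing the player limit as the result cap, and records the results and success flag.
; Session selection, joining and a misspelled "SeverTravel" console command are unconnected and never run.
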(event `Create Room`
  (params (`Max Player` :type Integer) (`Lan/Internet` :type Boolean))
  (bind _output_get (set `self.Max Player` `Max Player`))
  (bind _output_get_2 (set `self.Lan / Internet` `Lan/Internet`))
  (`CreateSessionCallbackProxy.CreateSession` (`GameplayStatics.GetPlayerController` 0) _output_get _output_get_2
    (:`OnSuccess`
      (`GameplayStatics.OpenLevel` "FirstPersonExampleMap" true "Listen"))))

(event `Find Room`
  (`KismetArrayLibrary.Array_Clear` (`self.Arr Sessions`))
  (bind _results (`FindSessionsCallbackProxy.FindSessions` (`GameplayStatics.GetPlayerController` 0) (`self.Max Player`) (`self.Lan / Internet`))
    (:`OnSuccess`
      (set `self.Arr Sessions` _results)
      (set `self.Find Success` true)
      (`KismetSystemLibrary.PrintString` "Hello" true true (struct :`G` 0.66 :`B` 1.0 :`A` 1.0) 10.0))
    (:`OnFailure`
      (set `self.Find Success` false))))