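; MyGameMode is a game mode Blueprint that persists account and password text through a MySaveGame object.
; CreateSaveGame loads the save slot if it exists, otherwise creates and writes a new one, copying both fields into the game mode's variables.
; SaveMySaveGame writes those variables back to the slot.
; BeginPlay is empty and the in-file CreateSaveGame call is unconnected, so nothing here triggers loading.
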(event `Create Save Game`
  (bind _returnvalue (`GameplayStatics.DoesSaveGameExist` "SaveSlot"))
  (if _returnvalue
    (bind _returnvalue_2 (`GameplayStatics.LoadGameFromSlot` "SaveSlot"))
    (bind _asmy_save_game (cast `/Game/BluePrint/Character/MySaveGame` _returnvalue_2))
    (set `self.MySaveGame` _asmy_save_game)
    (set `self.Txt Account` (`/Game/BluePrint/Character/MySaveGame.Txt_Account` (`self.MySaveGame`)))
    (set `self.Txt Pass` (`/Game/BluePrint/Character/MySaveGame.Txt_Pass` (`self.MySaveGame`)))
    (else
      (bind _returnvalue_3 (`GameplayStatics.CreateSaveGameObject` "/Game/BluePrint/Character/MySaveGame.MySaveGame_C"))
      (set `self.MySaveGame` _returnvalue_3)
      (set `self.Txt Account` (`/Game/BluePrint/Character/MySaveGame.Txt_Account` (`self.MySaveGame`)))
      (set `self.Txt Pass` (`/Game/BluePrint/Character/MySaveGame.Txt_Pass` (`self.MySaveGame`)))
      (`GameplayStatics.SaveGameToSlot` (`self.MySaveGame`) "SaveSlot"))))

(event `SaveMySaveGame`
  (set `/Game/BluePrint/Character/MySaveGame.Txt_Account` (`self.Txt Account`) (`self.MySaveGame`))
  (set `/Game/BluePrint/Character/MySaveGame.Txt_Pass` (`self.Txt Pass`) (`self.MySaveGame`))
  (`GameplayStatics.SaveGameToSlot` (`self.MySaveGame`) "SaveSlot"))

(event `self.ReceiveBeginPlay`)

(fn `UserConstructionScript`)